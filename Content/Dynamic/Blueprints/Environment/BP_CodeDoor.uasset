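; BP_CodeDoor is a locked exit that ends the level once the matching key has been delivered to it.
; A BP_KeyPickup overlapping the Box sets HasKeys when its KeyID matches the door's PasscodeID.
; When BP_BodyChar overlaps the Trigger with HasKeys set, the victory widget appears and, after a delay, LV_UknownFacility opens.
; Without the key, the Trigger only prints a hint about needing shapes.
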(event `self.Trigger.OnComponentBeginOverlap`
  (params (OverlappedComponent :type "PrimitiveComponent Object Reference") (OtherActor :type "Actor Object Reference") (OtherComp :type "PrimitiveComponent Object Reference") (OtherBodyIndex :type Integer) (bFromSweep :type Boolean) (SweepResult :type "HitResult Structure (by ref)"))
  (cast `/Game/Dynamic/Blueprints/Characters/BodyChar/BP_BodyChar` OtherActor)
  (if (`self.HasKeys?`)
    (bind _returnvalue (`|CreateWidget` "/Game/Dynamic/Blueprints/WBP_Victory.WBP_Victory_C"))
    (`UserWidget.AddToViewport` _returnvalue 0)
    (`KismetSystemLibrary.Delay` 5.0)
    (`GameplayStatics.OpenLevelBySoftObjectPtr` "/Game/Dynamic/Levels/LV_UknownFacility.LV_UknownFacility")
    (else
      (`KismetSystemLibrary.PrintString` "Need Ominous shapes"))))

(event `self.Box.OnComponentBeginOverlap`
  (params (OverlappedComponent :type "PrimitiveComponent Object Reference") (OtherActor :type "Actor Object Reference") (OtherComp :type "PrimitiveComponent Object Reference") (OtherBodyIndex :type Integer) (bFromSweep :type Boolean) (SweepResult :type "HitResult Structure (by ref)"))
  (bind _asbp_key_pickup (cast `/Game/Dynamic/Blueprints/Environment/BP_KeyPickup` OtherActor))
  (if (== (`/Game/Dynamic/Blueprints/Environment/BP_KeyPickup.KeyID` _asbp_key_pickup) (`self.PasscodeID`))
    (set `self.HasKeys?` true)))

(fn `UserConstructionScript`)